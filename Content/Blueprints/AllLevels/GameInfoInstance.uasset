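; Game instance that manages front-end menu widgets and multiplayer session hosting, joining and destruction.
; A PlayerSettingsSave check opens the main menu, or the options menu on first run; most widgets are cached for reuse.
; Hosting shows a loading screen, creates a session and opens FirstPersonMap as a listen server, while joining uses a search result.
; Session, network and travel failures route to DisplayErrorMessege, but it and both error-to-string helpers are empty stubs.
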(event Custom|ShowMainMenu
  (bind _returnvalue (Game|GetPlayerController 0))
  (Utilities|IsValid (Variables|Default|GetWB_MainMenu)
    (:Is%20Valid
      _)
    (:Is%20Not%20Valid
      (bind _returnvalue_2 (UserInterface|CreateWidget "/Game/UI/MainManu/MainMenu.MainMenu_C" _returnvalue))
      (Variables|Default|SetWB_MainMenu _returnvalue_2)))
  (UserInterface|Viewport|AddtoViewport (Variables|Default|GetWB_MainMenu) 0)
  (Variables|/Script/Engine.PlayerController|SetbShowMouseCursor _returnvalue true))

(event Custom|ShowLoadingScreen
  (Utilities|IsValid (Variables|Default|GetWB_LoadingScreen)
    (:Is%20Valid
      _)
    (:Is%20Not%20Valid
      (bind _returnvalue (UserInterface|CreateWidget "/Game/UI/AllLevels/LoadingScreen.LoadingScreen_C" (Game|GetPlayerController 0)))
      (Variables|Default|SetWB_LoadingScreen _returnvalue)))
  (UserInterface|Viewport|AddtoViewport (Variables|Default|GetWB_LoadingScreen) 0))

(event Custom|JoinServer
  (params (SessionToJoin :type Blueprint%20Session%20Result%20Structure))
  (CallFunction|ShowLoadingScreen)
  (|JoinSession (Game|GetPlayerController 0) SessionToJoin
    (:OnFailure
      (Utilities|DisplayErrorMessege "Failed To JoinSession"))))

(event Custom|ShowOptionsMenu
  (Utilities|IsValid (Variables|Default|GetWB_OptionsMenu)
    (:Is%20Valid
      _)
    (:Is%20Not%20Valid
      (bind _returnvalue (UserInterface|CreateWidget "/Game/UI/MainManu/OptionsMenu.OptionsMenu_C" (Game|GetPlayerController 0)))
      (Variables|Default|SetWB_OptionsMenu _returnvalue)))
  (UserInterface|Viewport|AddtoViewport (Variables|Default|GetWB_OptionsMenu) 0)
  (if (Variables|Default|GetCreatedSaveFile)
    (Default|HideRequestText (Variables|Default|GetWB_OptionsMenu))))

(event Custom|DestroySessionCaller
  (params (PlayerController :type Player%20Controller%20Object%20Reference))
  (|DestroySession PlayerController))

(event Custom|ShowServerMenu
  (bind _returnvalue (UserInterface|CreateWidget "/Game/UI/MainManu/ServerMenu.ServerMenu_C" (Game|GetPlayerController 0)))
  (UserInterface|Viewport|AddtoViewport _returnvalue 0))

(event Custom|CheckForSaveGame
  (bind _returnvalue (SaveGame|DoesSaveGameExist (Variables|Default|GetPlayerSettingsSave)))
  (if _returnvalue
    (CallFunction|ShowMainMenu)
    (Variables|Default|SetCreatedSaveFile true)
    (else
      (CallFunction|ShowOptionsMenu)
      (Variables|/Script/Engine.PlayerController|SetbShowMouseCursor (Game|GetPlayerController 0) false))))

(event Custom|ShowHostMenu
  (Utilities|IsValid (Variables|Default|GetWB_HostMenu)
    (:Is%20Valid
      _)
    (:Is%20Not%20Valid
      (bind _returnvalue (UserInterface|CreateWidget "/Game/UI/MainManu/HostMenu.HostMenu_C" (Game|GetPlayerController 0)))
      (Variables|Default|SetWB_HostMenu _returnvalue)))
  (UserInterface|Viewport|AddtoViewport (Variables|Default|GetWB_HostMenu) 0))

(event Custom|LaunchLobby
  (params (NumberOfPlayer :type Integer) (EnableLan? :type Boolean) (ServerName :type Text))
  (Variables|ServerSettings|SetMaxPlayers NumberOfPlayer)
  (Variables|ServerSettings|SetServerName ServerName)
  (CallFunction|ShowLoadingScreen)
  (|Session (Game|GetPlayerController 0) (Variables|ServerSettings|GetMaxPlayers) EnableLan?
    (:OnSuccess
      (Game|OpenLevel(byObjectReference) "/Game/Maps/FirstPersonMap.FirstPersonMap" true "listen"))
    (:OnFailure
      (Utilities|DisplayErrorMessege "Failed To Create Session"))))

(event EventHandleNetworkError
  (params (FailureType :type ENetworkFailure%20Enum :default "NetDriverAlreadyExists") (bIsServer :type Boolean))
  (Utilities|DisplayErrorMessege (CallFunction|NetErrortoString FailureType)))

(event EventHandleTravelError
  (params (FailureType :type ETravelFailure%20Enum :default "NoLevel"))
  (Utilities|DisplayErrorMessege (CallFunction|TravelErrortoString FailureType)))

(fn NetErrortoString
  (params (FailureType :type ENetworkFailure%20Enum :default "NetDriverAlreadyExists"))
  (return ""))

(fn TravelErrortoString
  (params (FailureType :type ETravelFailure%20Enum :default "NoLevel"))
  (return ""))