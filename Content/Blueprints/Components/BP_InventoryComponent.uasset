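; Inventory component that tracks item amounts by type in an Items array.
; AddItem raises the amount of a matching existing entry, while ConsumeItem lowers it and returns true only when enough is held.
; Both record the changed entry in LastSetItem, whose RepNotify calls OnItemCountChanged to announce the new count.
; BeginPlay assigns three hardcoded item structs to LastSetItem without writing them into Items.
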(event EventBeginPlay
  (Variables|Default|SetLastSetItem (Utilities|Struct|MakeItemStructure 10 "NewEnumerator1"))
  (Variables|Default|SetLastSetItem (Utilities|Struct|MakeItemStructure 0 "NewEnumerator2"))
  (Variables|Default|SetLastSetItem (Utilities|Struct|MakeItemStructure 40 "NewEnumerator0")))

(fn ConsumeItem
  (params (ItemStructure :type Item%20Structure%20Structure))
  (bind (_amount _itemtype) (Utilities|Struct|BreakItemStructure ItemStructure))
  (for (_array_element _array_index) (Variables|Default|GetItems)
    (if (Utilities|Enum|Equal(Enum) (.ItemType (Utilities|Struct|BreakItemStructure _array_element)) _itemtype)
      (if (>= (.Amount (Utilities|Struct|BreakItemStructure _array_element)) _amount)
        (bind _structout (Utilities|Struct|SetmembersinItemStructure _array_element (- (.Amount (Utilities|Struct|BreakItemStructure _array_element)) _amount)))
        (bind _output_get (Variables|Default|SetLastSetItem _structout))
        (Utilities|Array|SetArrayElem (Variables|Default|GetItems) _array_index _output_get)
        (return true)
        (else
          (return false))))))

(fn AddItem
  (params (ItemStructure :type Item%20Structure%20Structure))
  (bind (_amount _itemtype) (Utilities|Struct|BreakItemStructure ItemStructure))
  (for (_array_element _array_index) (Variables|Default|GetItems)
    (if (Utilities|Enum|Equal(Enum) (.ItemType (Utilities|Struct|BreakItemStructure _array_element)) _itemtype)
      (bind _structout (Utilities|Struct|SetmembersinItemStructure _array_element (+ (.Amount (Utilities|Struct|BreakItemStructure _array_element)) _amount)))
      (bind _output_get (Variables|Default|SetLastSetItem _structout))
      (Utilities|Array|SetArrayElem (Variables|Default|GetItems) _array_index _output_get)
      (return))))

(fn OnRepLastSetItem
  (Default|CallOnItemCountChanged (Variables|Default|GetLastSetItem)))